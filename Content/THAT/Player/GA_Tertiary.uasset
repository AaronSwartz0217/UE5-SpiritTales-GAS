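; GA_Tertiary is a player Gameplay Ability that gives BP_PlayerCharacter a one-second burst of extreme walk speed, with debug prints.
; On activation, a DrawDebugs flag gates the boost, and a Button flag gates caching of the original MaxWalkSpeed.
; After the delay, or immediately without DrawDebugs, it ends the ability, restores the cached speed and clears Button.
; The character's IsAC mirrors the ability's active state at start and end.
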(event `self.K2_ActivateAbility`
  (bind _asbp_player_character (cast `/Game/THAT/BP_PlayerCharacter` (`self.GetAvatarActorFromActorInfo`)))
  (set `/Game/THAT/BP_PlayerCharacter.IsAC` (`AbilitySystemBlueprintLibrary.IsGameplayAbilityActive` self) _asbp_player_character)
  (if (`self.bDrawDebugs`)
    (bind _asbp_player_character_2 (cast `/Game/THAT/BP_PlayerCharacter` (`self.GetAvatarActorFromActorInfo`)))
    (if (`self.button`)
      (bind _charactermovement (`Character.CharacterMovement` _asbp_player_character_2))
      (set `self.speedGAS` (`CharacterMovementComponent.MaxWalkSpeed` _charactermovement)))
    (set `CharacterMovementComponent.MaxWalkSpeed` 10000.0 _charactermovement)
    (`KismetSystemLibrary.PrintString` "TE")
    (`KismetSystemLibrary.PrintString` (`|GetEnumeratorNameAsString` (`CharacterMovementComponent.MovementMode` _charactermovement)))
    (`KismetSystemLibrary.Delay` 1.0))
  (`self.K2_EndAbility`)
  (set `CharacterMovementComponent.MaxWalkSpeed` (`self.speedGAS`) _charactermovement)
  (`KismetSystemLibrary.PrintString` "重置")
  (set `self.button` false)
  (bind _asbp_player_character_3 (cast `/Game/THAT/BP_PlayerCharacter` (`self.GetAvatarActorFromActorInfo`)))
  (set `/Game/THAT/BP_PlayerCharacter.IsAC` (`AbilitySystemBlueprintLibrary.IsGameplayAbilityActive` self) _asbp_player_character_3))