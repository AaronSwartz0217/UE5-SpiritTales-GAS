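; GA_Primary is the player's primary Gameplay Ability, apparently a melee attack with no hit detection or damage yet.
; A FlipFlop alternates between two montages, and the ability ends when the montage completes, blends out, is interrupted or is cancelled.
; In parallel, it waits for the Player.Primary gameplay event and draws a debug sphere of hitbox radius in front of the avatar.
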(event `self.K2_ActivateAbility`
  (bind _returnvalue (`self.GetAvatarActorFromActorInfo`))
  (bind _bdrawdebugs (`self.bDrawDebugs`)
    (:`then`
      (if _bdrawdebugs
        (`KismetSystemLibrary.PrintString` "GA")))
    (:`else`
      _))
  (`|ExecutionSequence`
    (:`then_0`
      (`/Engine/EditorBlueprintResources/StandardMacros.FlipFlop`
        (:`A`
          (`AbilityTask_PlayMontageAndWait.CreatePlayMontageAndWaitProxy` "None" "/Game/GameAnimsPack/Animations/MT.MT"
            (:`OnCompleted`
              _)
            (:`OnBlendOut`
              _)
            (:`OnInterrupted`
              _)
            (:`OnCancelled`
              _))
          (`self.K2_EndAbility`))
        (:`B`
          (`AbilityTask_PlayMontageAndWait.CreatePlayMontageAndWaitProxy` "None" "/Game/GameAnimsPack/Animations/MT2.MT2"
            (:`OnCompleted`
              _)
            (:`OnBlendOut`
              _)
            (:`OnInterrupted`
              _)
            (:`OnCancelled`
              _))
          (`self.K2_EndAbility`))))
    (:`then_1`
      (`AbilityTask_WaitGameplayEvent.WaitGameplayEvent` (struct :`TagName` "CCTags.Events.Player.Primary") null
        (:`EventReceived`
          (`self.bDrawDebugs`
            (:`then`
              (`KismetSystemLibrary.DrawDebugSphere` (+ (`Actor.K2_GetActorLocation` _returnvalue) (+ (* (`Actor.GetActorForwardVector` _returnvalue) 100.0) (0.0 0.0 20.0))) (`self.HitBoxRadius`)))
            (:`else`)))))))